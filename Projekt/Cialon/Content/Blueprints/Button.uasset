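; Interactive button that the player presses with the action key while something overlaps its Box trigger.
; BeginPlay binds the key event, and box overlaps open and close a gate that controls whether it passes.
; A passed press plays a timeline that adds MoveX to the button's current world location each update, so movement accumulates.
; When the timeline finishes, it prints a debug string and calls CallButtonON.
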(event OnComponentEndOverlap(Box)
  (params (OtherActor :type Actor%20Object%20Reference) (OtherComp :type Primitive%20Component%20Object%20Reference) (OtherBodyIndex :type Integer))
  (Utilities|FlowControl|Gate true) ; enters at Close
)

(event OnComponentBeginOverlap(Box)
  (params (OtherActor :type Actor%20Object%20Reference) (OtherComp :type Primitive%20Component%20Object%20Reference) (OtherBodyIndex :type Integer) (bFromSweep :type Boolean) (SweepResult :type Hit%20Result%20Structure%20%28by%20ref%29))
  (Utilities|FlowControl|Gate true) ; enters at Open
)

(event Custom|Action_key_Event
  (Utilities|FlowControl|Gate true
    (:Exit
      (bind _move_x (Timeline|Timeline_0 Play)
        (:Update
          (Transformation|SetWorldLocation (Variables|Default|GetButton) (+ _move_x (Transformation|GetWorldLocation (Variables|Default|GetButton))) false false))
        (:Finished
          (Development|PrintString "Hello")
          (Default|CallButtonON))))))

(event EventBeginPlay
  (EventDispatchers|BindEventtoActionKey (delegate Custom|Action_key_Event)))

(fn ConstructionScript)