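; Interactive chest that swings its lid open when the player triggers the action key while the chest's Box volume is overlapped.
; On BeginPlay it binds to the ActionKey dispatcher on the player's ThirdPersonCharacter.
; Box overlaps open and close a Gate for that event, without filtering the overlapping actor.
; A DoOnce then plays a Timeline that drives the Top component's relative roll, so the chest opens only once.
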(event OnComponentBeginOverlap(Box)
  (params (OtherActor :type Actor%20Object%20Reference) (OtherComp :type Primitive%20Component%20Object%20Reference) (OtherBodyIndex :type Integer) (bFromSweep :type Boolean) (SweepResult :type Hit%20Result%20Structure%20%28by%20ref%29))
  (Utilities|FlowControl|Gate true) ; enters at Open
)

(event OnComponentEndOverlap(Box)
  (params (OtherActor :type Actor%20Object%20Reference) (OtherComp :type Primitive%20Component%20Object%20Reference) (OtherBodyIndex :type Integer))
  (Utilities|FlowControl|Gate true) ; enters at Close
)

(event Custom|DispatcherTest_Event_1
  (Utilities|FlowControl|Gate true
    (:Exit
      (Utilities|FlowControl|DoOnce false
        (:Completed
          (bind _open_chest (Timeline|Chest_Open_animation Play)
            (:Update
              (Transformation|SetRelativeRotation (Variables|Default|GetTop) (Math|Rotator|MakeRotator (+ _open_chest 0.0) 0.0 0.0) false false))))))))

(event EventBeginPlay
  (EventDispatchers|AssignDispatcherActionKey (.AsThird%20Person%20Character (Utilities|Casting|CastToThirdPersonCharacter (Game|GetPlayerCharacter 0))) (delegate Custom|DispatcherTest_Event_1)))

(fn ConstructionScript)